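; Interactive door that the third-person character or fly drone can toggle while inside its trigger box.
; Overlap events bind the interaction delegate and toggle that pawn's HUD prompt.
; Interaction runs TryOpen, which toggles the door if unlocked, or calls the empty CheckForKey hook if locked.
; A timeline lerps the cube between its start and EndPosition's location, flips IsOpened on finish, and auto-closes after a delay.
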(event `self.Box.OnComponentBeginOverlap`
  (params (OverlappedComponent :type "PrimitiveComponent Object Reference") (OtherActor :type "Actor Object Reference") (OtherComp :type "PrimitiveComponent Object Reference") (OtherBodyIndex :type Integer) (bFromSweep :type Boolean) (SweepResult :type "HitResult Structure (by ref)"))
  (bind _isinrange (`self.IsInRange`))
  ;[1 1 1] RangeDetection
  (bind _asthird_person_character (cast `/Game/RemedyTest/BP/ThirdPersonCharacter` OtherActor)
    (:`then`
      (bind _output_get (set `self.PlayerRef` _asthird_person_character))
      (if (not _isinrange)
        (add `/Game/RemedyTest/BP/ThirdPersonCharacter.OnPlayerInteraction` _output_get (delegate `InteractionButtonPressed`))
        (`/Game/RemedyTest/Widget/W_PlayerHud.ToggleInteractionPrompt` (`/Game/RemedyTest/BP/ThirdPersonCharacter.PlayerWidgetRef` _output_get) "NewEnumerator1")
        (set `self.IsInRange` true :!label _label)))
    (:`CastFailed`
      (bind _asbp_fly_drone (cast `/Game/RemedyTest/BP/Drone/BP_FlyDrone` OtherActor))
      (bind _output_get_2 (set `self.FlyDroneRef` _asbp_fly_drone))
      (if (not _isinrange)
        (add `/Game/RemedyTest/BP/Drone/BP_FlyDrone.OnFlyDroneInteraction` _output_get_2 (delegate `InteractionButtonPressed`))
        (`/Game/RemedyTest/Widget/W_DroneHud.ToggleInteractionInfo` (`/Game/RemedyTest/BP/Drone/BP_DroneBase.DroneHudRef` _output_get_2) "NewEnumerator1")
        (goto _label)))))

(event `self.Box.OnComponentEndOverlap`
  (params (OverlappedComponent :type "PrimitiveComponent Object Reference") (OtherActor :type "Actor Object Reference") (OtherComp :type "PrimitiveComponent Object Reference") (OtherBodyIndex :type Integer))
  (bind _isinrange (`self.IsInRange`))
  ;[1 1 1] RangeDetection
  (bind _asthird_person_character (cast `/Game/RemedyTest/BP/ThirdPersonCharacter` OtherActor)
    (:`then`
      (if _isinrange
        (remove `/Game/RemedyTest/BP/ThirdPersonCharacter.OnPlayerInteraction` _asthird_person_character (delegate `InteractionButtonPressed`))
        (`/Game/RemedyTest/Widget/W_PlayerHud.ToggleInteractionPrompt` (`/Game/RemedyTest/BP/ThirdPersonCharacter.PlayerWidgetRef` _asthird_person_character) "NewEnumerator1")
        (set `self.IsInRange` false :!label _label_2)))
    (:`CastFailed`
      (bind _asbp_fly_drone (cast `/Game/RemedyTest/BP/Drone/BP_FlyDrone` OtherActor))
      (if _isinrange
        (remove `/Game/RemedyTest/BP/Drone/BP_FlyDrone.OnFlyDroneInteraction` _asbp_fly_drone (delegate `InteractionButtonPressed`))
        (`/Game/RemedyTest/Widget/W_DroneHud.ToggleInteractionInfo` (`/Game/RemedyTest/BP/Drone/BP_DroneBase.DroneHudRef` _asbp_fly_drone) "NewEnumerator1")
        (goto _label_2)))))

(event `self.ReceiveBeginPlay`
  ;[1 1 1] Begin Play
  (set `self.StartPos` (`SceneComponent.RelativeLocation` (`self.Cube`)))
  (set `self.EndPos` (`SceneComponent.RelativeLocation` (`self.EndPosition`))))

(event `InteractionButtonPressed`
  (`self.TryOpen`))

(event `CheckForKey`
  ;[1 1 1] CheckForKey
)

(event `TryOpen`
  ;[1 1 1] TryOpen
  (if (`self.IsLocked`)
    (`self.CheckForKey`)
    (else
      (`self.ToggleDoor`))))

(event `OpenDoor`
  ;[1 1 1] Open / Close door
  (if (not (`self.IsOpened`))
    (bind (_direction _newtrack_0) (`Timeline|DoorOpenClose` :!via `PlayFromStart` :!label _label_3)
      (:`Update`
        (`SceneComponent.K2_SetRelativeLocation` (`self.Cube`) (`KismetMathLibrary.VLerp` (`self.StartPos`) (`self.EndPos`) _newtrack_0) false false))
      (:`Finished`
        (set `self.IsOpened` (not (`self.IsOpened`)))
        (`self.OnFinished`)))))

(event `ToggleDoor`
  ;[1 1 1] Open / Close door
  (if (`self.IsOpened`)
    (goto _label_3 :!via `Reverse`)
    (else
      (goto _label_3 :!via `PlayFromStart`))))

(event `CloseDoor`
  ;[1 1 1] Open / Close door
  (if (`self.IsOpened`)
    (goto _label_3 :!via `Reverse`)))

(event `OnFinished`
  ;[1 1 1] Open / Close door
  (`KismetSystemLibrary.Delay` 2.0)
  (`self.CloseDoor`))

(fn `LockDoor`
  (set `self.IsLocked` true))

(fn `UnlockDoor`
  (set `self.IsLocked` false))

(fn `UserConstructionScript`
  (`parent.UserConstructionScript`))