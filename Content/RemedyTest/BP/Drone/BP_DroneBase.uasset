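; BP_DroneBase is a base drone pawn that the player can take control of and that detects nearby interactibles.
; ControlDrone hands the owner's controller to the drone and stores the owner, and the SpawnDrone input calls PossessPlayer on that owner to switch back.
; Box overlaps with BP_interactible actors fire empty in-range and out-of-range events, apparently left for child drones to override.
; SetReferences stores the player HUD.
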(event `ControlDrone`
  (params (Owner :type "/Game/RemedyTest/BP/ThirdPersonCharacter Object Reference"))
  ;[1 1 1] Possession
  (`Controller.Possess` (`self.GetController` Owner) self)
  (set `self.isPossessed` true)
  (set `self.PlayerOwner` Owner))

(event `InputAction|SpawnDrone`
  (params (Key :type "Key Structure"))
  ;[1 1 1] Possession
  (:`Pressed`
    (`/Game/RemedyTest/BP/ThirdPersonCharacter.PossessPlayer` (`self.PlayerOwner`))))

(event `self.Box.OnComponentBeginOverlap`
  (params (OverlappedComponent :type "PrimitiveComponent Object Reference") (OtherActor :type "Actor Object Reference") (OtherComp :type "PrimitiveComponent Object Reference") (OtherBodyIndex :type Integer) (bFromSweep :type Boolean) (SweepResult :type "HitResult Structure (by ref)"))
  ;[1 1 1] Interaction Range
  (bind _asbp_interactible (cast `/Game/RemedyTest/BP/Interactible/BP_interactible` OtherActor))
  (`self.OnDroneInRange` _asbp_interactible))

(event `self.Box.OnComponentEndOverlap`
  (params (OverlappedComponent :type "PrimitiveComponent Object Reference") (OtherActor :type "Actor Object Reference") (OtherComp :type "PrimitiveComponent Object Reference") (OtherBodyIndex :type Integer))
  ;[1 1 1] Interaction Range
  (bind _asbp_interactible (cast `/Game/RemedyTest/BP/Interactible/BP_interactible` OtherActor))
  (`self.OnDroneOutOfRange` _asbp_interactible))

(event `OnDroneInRange`
  (params (Interactible :type "/Game/RemedyTest/BP/Interactible/BP_interactible Object Reference"))
  ;[1 1 1] Interaction Range
)

(event `OnDroneOutOfRange`
  (params (Interactible :type "/Game/RemedyTest/BP/Interactible/BP_interactible Object Reference"))
  ;[1 1 1] Interaction Range
)

(fn `SetReferences`
  (params (PlayerHud :type "/Game/RemedyTest/Widget/W_PlayerHud Object Reference"))
  (set `self.PlayerHud` PlayerHud))

(fn `UserConstructionScript`)